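; BP_AiSoccer is an AI soccer player that positions itself around the ball relative to the opposing team's goal.
; BeginPlay caches the ball and a goal from another team.
; Each Tick, a dot product of player-to-ball and ball-to-goal directions picks the move.
; AI MoveTo targets a point just behind the ball when aligned, otherwise a rotated offset to its side, drawn as a debug sphere.
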(event Custom|PushBall
  (AI|AIMoveTo self (+ (* (* (Math|Vector|GetUnitDirection(Vector) (Transformation|GetActorLocation (Variables|Default|GetBallRef)) (Transformation|GetActorLocation (Variables|Default|GetGoalToScore))) -1.0) 1e+02) (Transformation|GetActorLocation (Variables|Default|GetBallRef))) 0 5.0 false))

(event Custom|SwitchSide
  (bind _ballref (Variables|Default|GetBallRef))
  (bind _ballref_2 (Variables|Default|GetBallRef))
  (bind _goaltoscore (Variables|Default|GetGoalToScore))
  (bind _returnvalue (Transformation|GetActorLocation _ballref))
  (bind _returnvalue_2 (Transformation|GetActorLocation _ballref_2))
  (bind _returnvalue_3 (Transformation|GetActorLocation _goaltoscore))
  (bind _returnvalue_4 (Math|Vector|GetUnitDirection(Vector) _returnvalue_2 _returnvalue_3))
  (bind _returnvalue_5 (Math|Vector|RotateVectorAroundAxis _returnvalue_4 1e+02 "0.000000,0.000000,1.000000"))
  (bind _returnvalue_6 (* _returnvalue_5 2e+02))
  (bind _returnvalue_7 (+ _returnvalue_6 _returnvalue))
  (Rendering|Debug|DrawDebugSphere _returnvalue_7 1e+02 12 "(R=1.000000,G=1.000000,B=1.000000,A=1.000000)" 1.0 1.0)
  (AI|AIMoveTo self _returnvalue_7 0 5.0 false))

(event EventBeginPlay
  (bind _returnvalue (Actor|GetActorOfClass "/Game/BP_Ball.BP_Ball_C"))
  (Variables|Default|SetBallRef _returnvalue)
  (bind _outactors (Actor|GetAllActorsOfClass "/Game/BP_Goal.BP_Goal_C"))
  (for _array_element _outactors
    (if (Utilities|Enum|NotEqual(Enum) (Variables|Default|GetTeam) (Variables|/Game/BP_Goal.BP_Goal_C|GetTeam _array_element))
      (Variables|Default|SetGoalToScore _array_element))))

(event Collision|EventActorBeginOverlap
  (params (OtherActor :type Actor%20Object%20Reference)))

(event EventTick
  (params (DeltaSeconds :type Float%20%28single-precision%29))
  (bind _output_get (Variables|Default|SetWellPlaced (>= (Math|Vector|DotProduct (Math|Vector|GetUnitDirection(Vector) (Transformation|GetActorLocation (Variables|Default|GetBallRef)) (Transformation|GetActorLocation (Variables|Default|GetGoalToScore))) (Math|Vector|GetUnitDirection(Vector) (Transformation|GetWorldLocation (Variables|Collision|GetCapsuleComponent)) (Transformation|GetActorLocation (Variables|Default|GetBallRef)))) 0.0)))
  (if _output_get
    (CallFunction|PushBall)
    (else
      (CallFunction|SwitchSide))))

(fn ConstructionScript)