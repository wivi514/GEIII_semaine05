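; Soccer manager actor that keeps score for teams A and B and resets the ball after each goal.
; On BeginPlay it creates the SoccerWidget, passes itself as a reference and adds it to the viewport.
; The Score event increments the given team's count, plays an explosion sound and, after a short delay, calls SpawnBall.
; SpawnBall teleports the existing BP_Ball's sphere to the spawn arrow rather than spawning a new actor.
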(event Custom|Score
  (params (Team :type String))
  (switch string Team
    (:A
      (Math|Integer|IncrementInt (Variables|Default|GetScoreTeamA)
        (:%20%20
          _)))
    (:B
      (Math|Integer|IncrementInt (Variables|Default|GetScoreTeamB)
        (:%20%20
          _))))
  (Audio|PlaySound2D "/Game/StarterContent/Audio/Explosion01.Explosion01" 1.0 1.0 0.0 0 0)
  (Utilities|FlowControl|Delay 2.0)
  (CallFunction|SpawnBall))

(event Custom|Spawn%20Ball
  (bind _returnvalue (Actor|GetActorOfClass "/Game/BP_Ball.BP_Ball_C"))
  (Transformation|SetWorldLocation (Variables|/Game/BP_Ball.BP_Ball_C|GetSphere _returnvalue) (Transformation|GetWorldLocation (Variables|Default|GetArrowBallSpawn_0)) false true))

(event EventBeginPlay
  (bind _returnvalue (UserInterface|CreateWidget "/Game/SoccerWidget.SoccerWidget_C"))
  (Variables|/Game/SoccerWidget.SoccerWidget_C|SetSM_Ref _returnvalue self)
  (UserInterface|Viewport|AddtoViewport _returnvalue 0))

(fn ConstructionScript)